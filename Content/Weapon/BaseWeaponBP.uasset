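; BaseWeaponBP is a base weapon actor that the player can pick up through proximity and an interact input.
; Overlap with its Sphere by a MyCharacter stores that character, shows the Widget, sets CanWePick and enables input on the actor for player controller 0.
; Leaving the sphere reverses the prompt, flag and input.
; While pickable, the ItemInteration action calls PickUp on the stored character and prints a debug string.
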(event `self.Sphere.OnComponentBeginOverlap`
  (params (OverlappedComponent :type "PrimitiveComponent Object Reference") (OtherActor :type "Actor Object Reference") (OtherComp :type "PrimitiveComponent Object Reference") (OtherBodyIndex :type Integer) (bFromSweep :type Boolean) (SweepResult :type "HitResult Structure (by ref)"))
  (bind _asmy_character (cast `/Game/Resources/Character/MyCharacter` OtherActor))
  (set `self.myCharacterRef` _asmy_character)
  (`SceneComponent.SetVisibility` (`self.Widget`) true false)
  (set `self.canWePick` true)
  (`self.EnableInput` (`GameplayStatics.GetPlayerController` 0)))

(event `self.Sphere.OnComponentEndOverlap`
  (params (OverlappedComponent :type "PrimitiveComponent Object Reference") (OtherActor :type "Actor Object Reference") (OtherComp :type "PrimitiveComponent Object Reference") (OtherBodyIndex :type Integer))
  (cast `/Game/Resources/Character/MyCharacter` OtherActor)
  (`SceneComponent.SetVisibility` (`self.Widget`) false false)
  (set `self.canWePick` false)
  (`self.DisableInput` (`GameplayStatics.GetPlayerController` 0)))

(event `InputAction|ItemInteration`
  (params (Key :type "Key Structure"))
  (:`Pressed`
    (if (`self.canWePick`)
      (`/Game/Resources/Character/MyCharacter.PickUp` (`self.myCharacterRef`) null)
      (`KismetSystemLibrary.PrintString` "PickUp"))))

(fn `UserConstructionScript`)